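; BP_PitchCharacter is a player character Blueprint that holds pitch data: profile name and image, protagonist icon, and a combined set of text responses such as title, genre and quote.
; Server and multicast events are set up to replicate the profile, but UpdateUserProfile only prints the name and its authority switch is disconnected.
; Setting, music and critic opinion updaters are empty stubs, and the scene print functions output debug strings.
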(event `Update User Profile`
  (params (InputName :type String) (InputImage :type "Texture2D Object Reference"))
  (`KismetSystemLibrary.PrintString` InputName true false))

(event `Server_UpdateUserProfile`
  (`self.Multicast_UpdateUserProfile`))

(event `Multicast_UpdateUserProfile`
  (bind _output_get (set `self.Name` (stale `Update User Profile` InputName)))
  (set `self.Img` (stale `Update User Profile` InputImage))
  (`KismetSystemLibrary.PrintString` _output_get true false))

(fn `Get Name of me`
  (returns (NewParam :type String))
  (return "PlayerCharacter"))

(fn `PrintConstructedScene`
  (`KismetSystemLibrary.PrintString` "Hello")
  (`KismetSystemLibrary.PrintString` "Hello")
  (`KismetSystemLibrary.PrintString` (`KismetSystemLibrary.GetPathName` null))
  (`KismetSystemLibrary.PrintString` "Hello")
  (`KismetSystemLibrary.PrintString` "Hello")
  (`KismetSystemLibrary.PrintString` (`KismetSystemLibrary.GetPathName` null))
  (`KismetSystemLibrary.PrintString` "Hello")
  (`KismetSystemLibrary.PrintString` (`KismetSystemLibrary.GetPathName` null))
  (`KismetSystemLibrary.PrintString` (`KismetSystemLibrary.GetObjectName` null))
  (`KismetSystemLibrary.PrintString` "Hello")
  (`KismetSystemLibrary.PrintString` "Hello")
  (`KismetSystemLibrary.PrintString` "Hello"))

(fn `PrintOnlySettings`
  (`KismetSystemLibrary.PrintString` "Hello")
  (`KismetSystemLibrary.PrintString` (`KismetSystemLibrary.GetObjectName` null)))

(fn `Update Critic Opinion`
  (params (`Critic Opinion` :type String)))

(fn `Update Music`
  (params (`Music Name` :type String) (`Music Icon` :type "Texture2D Object Reference") (`Music Sound` :type "SoundMix Object Reference")))

(fn `Update Protagonist`
  (params (`Protagonist Icon` :type "Texture2D Object Reference"))
  (set `self.Protag Icon` `Protagonist Icon`))

(fn `Update Setting`
  (params (`Setting Name` :type String) (`Setting Icon` :type "Texture2D Object Reference")))

(fn `Update Whole State`
  (params (Title :type String) (`Protagonist Name` :type String) (`Protagonist Occupation` :type String) (`Critic Opinion` :type String) (Genre :type String) (Quote :type String))
  (set `self.CombineResponses` (make `/Game/Characters/CombinedResponsesFromParent` Title `Protagonist Name` `Protagonist Occupation` `Critic Opinion` Genre Quote)))

(fn `UserConstructionScript`)