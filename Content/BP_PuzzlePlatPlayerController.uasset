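; BP_PuzzlePlatPlayerController is a player controller that holds and updates a user profile, consisting of a name and an image.
; UpdateUserProfile_Controller sets Name, then calls the multicast directly on authority or routes through a server event on remote.
; The multicast event sets Name, clears Image to None rather than applying an input image, and prints the name on screen.
; GetNameChar exposes the stored Name.
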(event `Update User Profile_Controller`
  (params (InputName :type String) (InputImage :type "Texture2D Object Reference"))
  (set `self.Name` InputName)
  (`/Engine/EditorBlueprintResources/ActorMacros.Switch Has Authority`
    (:`Authority`
      (`self.Multicast_UpdateUserProfile`))
    (:`Remote`
      (`self.Server_UpdateUserProfile`))))

(event `Server_UpdateUserProfile`
  (`self.Multicast_UpdateUserProfile`))

(event `Multicast_UpdateUserProfile`
  (bind _output_get (set `self.Name` (stale `Update User Profile_Controller` InputName)))
  (set `self.Image` null)
  (`KismetSystemLibrary.PrintString` _output_get true false))

(fn `GetNameChar`
  (returns (Name :type String))
  (return (`self.Name`)))

(fn `UserConstructionScript`)