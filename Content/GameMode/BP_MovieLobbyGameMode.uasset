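; Game mode for a movie lobby that stores player choices and compiles them into movie poster data.
; Update functions save the text responses, setting name and icon, and protagonist avatar.
; UpdateStructForMoviePoster merges these into CompiledPoster, using the genre as a map key to pick background and props.
; Print functions output stored values for debugging, while UpdatePlayerResponses and PrintOnlyMusic are empty stubs.
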(event `Update Player Responses`
  (params (Answer :type String)))

(event `Print Player Responses`
  (`KismetSystemLibrary.PrintString` "Hello, from game mode"))

(fn `PrintedConstructionScene`
  (bind (_combineresponse_gamemode_title _combineresponse_gamemode_protagonistname _combineresponse_gamemode_protagonistoccupation _combineresponse_gamemode_criticopinion _combineresponse_gamemode_genre _combineresponse_gamemode_quote) (break `/Game/Characters/CombinedResponsesFromParent` (`self.CombineResponse_GameMode`)))
  (`KismetSystemLibrary.PrintString` _combineresponse_gamemode_title)
  (`KismetSystemLibrary.PrintString` _combineresponse_gamemode_protagonistname)
  (`KismetSystemLibrary.PrintString` _combineresponse_gamemode_protagonistoccupation)
  (`KismetSystemLibrary.PrintString` _combineresponse_gamemode_criticopinion)
  (`KismetSystemLibrary.PrintString` _combineresponse_gamemode_genre)
  (`KismetSystemLibrary.PrintString` _combineresponse_gamemode_quote))

(fn `PrintOnlyAvatar`
  (`KismetSystemLibrary.PrintString` (`KismetSystemLibrary.GetPathName` (`self.Protagonist Icon`))))

(fn `PrintOnlyMusic`)

(fn `PrintOnlySettings`
  (bind (_settingsdata_settingname _settingsdata_settingicon) (break `/Game/Characters/SettingsData` (`self.SettingsData`)))
  (`KismetSystemLibrary.PrintString` _settingsdata_settingname)
  (`KismetSystemLibrary.PrintString` (`KismetSystemLibrary.GetObjectName` _settingsdata_settingicon)))

(fn `Update Avatar Icon`
  (params (`Avatar Icon` :type "Texture2D Object Reference"))
  (set `self.Protagonist Icon` `Avatar Icon`))

(fn `UpdatePrincipleWidgetResponses`
  (params (Title :type String) (`Protagonist Name` :type String) (`Protagonist Occupation` :type String) (`Critic Opinion` :type String) (Genre :type String) (Quote :type String))
  (set `self.CombineResponse_GameMode` (make `/Game/Characters/CombinedResponsesFromParent` Title `Protagonist Name` `Protagonist Occupation` `Critic Opinion` Genre Quote)))

(fn `UpdateSettings`
  (params (`Settings Name` :type String) (`Settings Icon` :type "Texture2D Object Reference"))
  (set `self.SettingsData` (make `/Game/Characters/SettingsData` `Settings Name` `Settings Icon`)))

(fn `UpdateStructForMoviePoster`
  (params (NewParam :type String))
  (bind (_combineresponse_gamemode_title _combineresponse_gamemode_protagonistname _combineresponse_gamemode_protagonistoccupation _combineresponse_gamemode_criticopinion _combineresponse_gamemode_genre _combineresponse_gamemode_quote) (break `/Game/Characters/CombinedResponsesFromParent` (`self.CombineResponse_GameMode`)))
  (bind (_settingsdata_settingname _settingsdata_settingicon) (break `/Game/Characters/SettingsData` (`self.SettingsData`)))
  (set `self.CompiledPoster` (make `/Game/Characters/CompiledPoster` _combineresponse_gamemode_criticopinion _combineresponse_gamemode_title _combineresponse_gamemode_quote (`self.Protagonist Icon`) (`BlueprintMapLibrary.Map_Find` (`self.BackgroundGenres`) _combineresponse_gamemode_genre) _settingsdata_settingicon (`BlueprintMapLibrary.Map_Find` (`self.Props`) _combineresponse_gamemode_genre))))

(fn `UserConstructionScript`)